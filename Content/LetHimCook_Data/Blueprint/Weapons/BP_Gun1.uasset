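; BP_Gun1 is a pistol weapon Blueprint that fires food actors.
; On BeginPlay it enables player input and adds a crosshair widget; IA_Shoot then plays a world camera shake, spawns BP_Food at the Arrow and plays a plop sound.
; Tick draws a debug trace from the muzzle along the mesh's right vector, without using the hit.
; Logic yawing the pistol toward a camera-center trace is present but unconnected.
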(event Input|EnhancedActionEvents|EnhancedInputActionIA_Shoot
  (params (ActionValue :type Float%20%28double-precision%29) (ElapsedSeconds :type Float%20%28double-precision%29) (TriggeredSeconds :type Float%20%28double-precision%29) (InputAction :type Input%20Action%20Object%20Reference :default "/Game/LetHimCook_Data/Blueprint/Inputs/IA_Shoot.IA_Shoot"))
  (bind _arrow (Variables|Default|GetArrow))
  (bind _returnvalue (Transformation|GetWorldTransform _arrow))
  ;[1 1 1] Camera Shake
  (:Started
    (Camera|PlayWorldCameraShake "/Game/LetHimCook_Data/Blueprint/Weapons/BP_ShootCameraShake.BP_ShootCameraShake_C" (Transformation|GetActorLocation) 0.0 3e+03 1.0 true)
    ;[1 1 1] Spawn Food
    (Game|SpawnActorfromClass "/Game/LetHimCook_Data/Blueprint/Weapons/BP_Food.BP_Food_C" (Math|Transform|MakeTransform (.location _returnvalue) (.rotation _returnvalue) "1.000000,1.000000,1.000000") "Undefined" "MultiplyWithRoot" 0 0)
    (Audio|PlaySoundatLocation "/Game/LetHimCook_Data/Audio/Plop.Plop" (.location _returnvalue) "0, 0, 0" 1.0 1.0 0.0 0 0 0 0)))

(event EventTick
  (params (DeltaSeconds :type Float%20%28single-precision%29))
  (bind _sk_pistol (Variables|Default|GetSK_Pistol))
  (bind _returnvalue (Transformation|GetSocketLocation _sk_pistol "Muzzle"))
  ;[1 1 1] Line Trace (Aim Location)
  (Collision|LineTraceByChannel _returnvalue (+ _returnvalue (* (Math|Vector|GetRightVector _sk_pistol) (Variables|Default|GetWeaponRange))) "TraceTypeQuery1" false 0 "ForOneFrame"))

(event EventBeginPlay
  ;[1 1 1] Enable Input
  (Input|EnableInput (Game|GetPlayerController 0))
  ;[1 1 1] Crosshair
  (bind _returnvalue (UserInterface|CreateWidget "/Game/LetHimCook_Data/Visuals/UI/WB_Crosshair.WB_Crosshair_C"))
  (UserInterface|Viewport|AddtoViewport _returnvalue 0))

(fn ConstructionScript)