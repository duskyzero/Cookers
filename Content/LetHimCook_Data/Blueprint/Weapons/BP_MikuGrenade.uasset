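; BP_MikuGrenade is a grenade weapon projectile with a ProjectileMovement component, which at this stage only prints a debug "Hello" when the projectile stops.
; The component-activated event is empty, and the construction script only calls its parent.
; Unconnected nodes would deactivate a component, enable physics on the capsule, and randomly rotate the static mesh, but they never execute.
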(event OnComponentActivated(ProjectileMovement)
  (params (Component :type Actor%20Component%20Object%20Reference) (bReset :type Boolean)))

(event OnProjectileStop(ProjectileMovement)
  (params (ImpactResult :type Hit%20Result%20Structure%20%28by%20ref%29))
  (Development|PrintString "Hello"))

(fn ConstructionScript
  (|CallParentFunction))