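; BP_Ammo is an ammo refill point that lets the chef top up the pistol on a key press.
; Box overlap with BP_Chef enables input on the actor, and any end overlap disables it.
; IA_PickItem finds the BP_WeaponPistol via GetActorOfClass and fills its current ammo to the total, or reports it full, with printed text and a sound either way.
; The actor stays in the world after use.
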(event OnComponentBeginOverlap(Box)
  (params (OverlappedComponent :type Primitive%20Component%20Object%20Reference) (OtherActor :type Actor%20Object%20Reference) (OtherComp :type Primitive%20Component%20Object%20Reference) (OtherBodyIndex :type Integer) (bFromSweep :type Boolean) (SweepResult :type Hit%20Result%20Structure%20%28by%20ref%29))
  ;[1 1 1] Check for player in range, If True = Enable Input
  (Utilities|Casting|CastToBP_Chef OtherActor)
  (Input|EnableInput (Game|GetPlayerController 0)))

(event OnComponentEndOverlap(Box)
  (params (OverlappedComponent :type Primitive%20Component%20Object%20Reference) (OtherActor :type Actor%20Object%20Reference) (OtherComp :type Primitive%20Component%20Object%20Reference) (OtherBodyIndex :type Integer))
  ;[1 1 1] Disable input when player not in range
  (Input|DisableInput (Game|GetPlayerController 0)))

(event Input|EnhancedActionEvents|EnhancedInputActionIA_PickItem
  (params (ActionValue :type Boolean) (ElapsedSeconds :type Float%20%28double-precision%29) (TriggeredSeconds :type Float%20%28double-precision%29) (InputAction :type Input%20Action%20Object%20Reference :default "/Game/LetHimCook_Data/Blueprint/Inputs/IA_PickItem.IA_PickItem"))
  ;[1 1 1] Reload
  (:Started
    (bind _returnvalue (Actor|GetActorOfClass "/Game/LetHimCook_Data/Blueprint/Weapons/BP_WeaponPistol.BP_WeaponPistol_C"))
    (if (== (- (Variables|/Game/LetHimCook_Data/Blueprint/Weapons/BP_WeaponPistol.BP_WeaponPistol_C|GetTotalAmmoCount _returnvalue) (Variables|/Game/LetHimCook_Data/Blueprint/Weapons/BP_WeaponPistol.BP_WeaponPistol_C|GetCurrentAmmoAmount _returnvalue)) 0)
      (Development|PrintString "Ammo Full" true true "(R=1.000000,G=0.304892,B=0.228494,A=1.000000)")
      (Audio|PlaySound2D "/Engine/VREditor/Sounds/UI/Dockable_Window_Drop.Dockable_Window_Drop" 1.0 1.0 0.0 0 0)
      (else
        (Variables|/Game/LetHimCook_Data/Blueprint/Weapons/BP_WeaponPistol.BP_WeaponPistol_C|SetCurrentAmmoAmount _returnvalue (+ (Variables|/Game/LetHimCook_Data/Blueprint/Weapons/BP_WeaponPistol.BP_WeaponPistol_C|GetCurrentAmmoAmount _returnvalue) (- (Variables|/Game/LetHimCook_Data/Blueprint/Weapons/BP_WeaponPistol.BP_WeaponPistol_C|GetTotalAmmoCount _returnvalue) (Variables|/Game/LetHimCook_Data/Blueprint/Weapons/BP_WeaponPistol.BP_WeaponPistol_C|GetCurrentAmmoAmount _returnvalue))))
        (Development|PrintString "Ammo Replenished" true true "(R=0.000000,G=1.000000,B=0.942305,A=1.000000)")
        ;[1 1 1] Play Sound
        (Audio|PlaySoundatLocation "/Engine/EditorSounds/Notifications/CompileSuccess.CompileSuccess" (Transformation|GetWorldLocation (Variables|Default|GetCube)) "0, 0, 0" 1.0 1.0 0.0 0 0 0 0)))))

(fn ConstructionScript)