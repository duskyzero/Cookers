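; BP_WeaponPlaceholder2 is a placeholder weapon that fires BP_MikuGrenade projectiles.
; On BeginPlay it enables input for player 0, removes all widgets and puts a WB_Crosshair on the viewport.
; When IA_Shoot starts, it spawns a grenade at the location and rotation of its Arrow component.
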(event Input|EnhancedActionEvents|EnhancedInputActionIA_Shoot
  (params (ActionValue :type Float%20%28double-precision%29) (ElapsedSeconds :type Float%20%28double-precision%29) (TriggeredSeconds :type Float%20%28double-precision%29) (InputAction :type Input%20Action%20Object%20Reference :default "/Game/LetHimCook_Data/Blueprint/Inputs/IA_Shoot.IA_Shoot"))
  (bind _arrow (Variables|Default|GetArrow))
  (bind _returnvalue (Transformation|GetWorldTransform _arrow))
  (:Started
    (Game|SpawnActorfromClass "/Game/LetHimCook_Data/Blueprint/Weapons/BP_MikuGrenade.BP_MikuGrenade_C" (Math|Transform|MakeTransform (.location _returnvalue) (.rotation _returnvalue) "1.000000,1.000000,1.000000") "Undefined" "MultiplyWithRoot" 0 0)))

(event EventBeginPlay
  ;[1 1 1] Enable Input
  (Input|EnableInput (Game|GetPlayerController 0))
  ;[1 1 1] Crosshair
  (Viewport|RemoveAllWidgets)
  (bind _returnvalue (UserInterface|CreateWidget "/Game/LetHimCook_Data/Visuals/UI/WB_Crosshair.WB_Crosshair_C"))
  (UserInterface|Viewport|AddtoViewport _returnvalue 0))

(fn ConstructionScript
  (|CallParentFunction))