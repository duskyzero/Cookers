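; BP_WeaponPistol is a pistol actor that launches BP_Food from its Arrow component, using up limited ammo.
; BeginPlay enables player input, replaces all widgets with a crosshair and draws a material to a render target.
; IA_Shoot spawns food with camera shake and sound, or signals when ammo is empty.
; Tick debug-draws a predicted projectile path from the Arrow and runs a muzzle line trace whose result is unused.
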(event Input|EnhancedActionEvents|EnhancedInputActionIA_Shoot
  (params (ActionValue :type Float%20%28double-precision%29) (ElapsedSeconds :type Float%20%28double-precision%29) (TriggeredSeconds :type Float%20%28double-precision%29) (InputAction :type Input%20Action%20Object%20Reference :default "/Game/LetHimCook_Data/Blueprint/Inputs/IA_Shoot.IA_Shoot"))
  (bind _arrow (Variables|Default|GetArrow))
  (bind _returnvalue (Transformation|GetWorldTransform _arrow))
  (:Started
    (if (== (Variables|Default|GetCurrentAmmoAmount) 0)
      (Audio|PlaySoundatLocation "/Engine/VREditor/Sounds/UI/Invalid_Action.Invalid_Action" (Transformation|GetWorldLocation (Variables|Default|GetSK_Pistol)) "0, 0, 0" 1.0 1.0 0.0 0 0 0 0)
      (Development|PrintString "Out of Ammo!" true true "(R=1.000000,G=0.000000,B=0.000000,A=1.000000)")
      (else
        (Camera|PlayWorldCameraShake "/Game/LetHimCook_Data/Blueprint/Weapons/BP_ShootCameraShake.BP_ShootCameraShake_C" (Transformation|GetActorLocation) 0.0 3e+03)
        (Game|SpawnActorfromClass "/Game/LetHimCook_Data/Blueprint/Weapons/BP_Food.BP_Food_C" (Math|Transform|MakeTransform (.location _returnvalue) (.rotation _returnvalue) "1.000000,1.000000,1.000000") "Undefined" "MultiplyWithRoot" 0 0)
        (Audio|PlaySoundatLocation "/Game/LetHimCook_Data/Audio/Plop.Plop" (.location _returnvalue) "0, 0, 0" 1.0 1.0 0.0 0 0 0 0)
        (bind _output_get (Variables|Default|SetCurrentAmmoAmount (- (Variables|Default|GetCurrentAmmoAmount) 1)))
        (Development|PrintString (Utilities|String|Append "Ammo Left : " (Utilities|String|ToString(Integer) _output_get)) true true "(R=0.161726,G=1.000000,B=0.411169,A=1.000000)")))))

(event EventTick
  (params (DeltaSeconds :type Float%20%28single-precision%29))
  (bind _sk_pistol (Variables|Default|GetSK_Pistol))
  (bind _arrow (Variables|Default|GetArrow))
  (bind _returnvalue (Transformation|GetSocketLocation _sk_pistol "Muzzle"))
  ;[1 1 1] Line Trace (Aim Location)
  (Collision|LineTraceByChannel _returnvalue (+ _returnvalue (* (Math|Vector|GetRightVector _sk_pistol) (Variables|Default|GetWeaponRange))) "TraceTypeQuery1" false 0 "None")
  (bind _predictresult (Class|GameplayStatics|BlueprintPredictProjectilePathAdvanced (Utilities|Struct|MakePredictProjectilePathParams (Transformation|GetWorldLocation _arrow) (* (Math|Vector|GetForwardVector (Transformation|GetWorldRotation _arrow)) "3000.000000,3000.000000,3000.000000") true 5.0 5.0 true "ECC_WorldStatic" "ObjectTypeQuery1" 0 2e+01 0.0 "ForOneFrame" 1.0 false))))

(event EventBeginPlay
  ;[1 1 1] Enable Input
  (Input|EnableInput (Game|GetPlayerController 0))
  ;[1 1 1] Crosshair
  (Viewport|RemoveAllWidgets)
  (bind _returnvalue (UserInterface|CreateWidget "/Game/LetHimCook_Data/Visuals/UI/WB_Crosshair.WB_Crosshair_C"))
  (UserInterface|Viewport|AddtoViewport _returnvalue 0)
  (Rendering|DrawMaterialtoRenderTarget 0 0))

(fn ConstructionScript
  (|CallParentFunction))