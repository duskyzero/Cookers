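; BP_MasterProjectile is a projectile Blueprint for weapon ammo, configured by an ammo data asset.
; On BeginPlay it synchronously loads AmmoDataAsset, casts it to DA_AmmoBase, and uses its Speed to set the ProjectileMovement velocity along local forward.
; It then gives the Sphere component a one-time random world rotation.
; The graph defines no hit or damage logic, and its construction script is empty.
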(event EventBeginPlay
  (bind _returnvalue (Utilities|LoadAssetBlocking (Variables|Default|GetAmmoDataAsset)))
  (bind _asda_ammo_base (Utilities|Casting|CastToDA_AmmoBase _returnvalue))
  (Game|Components|ProjectileMovement|SetVelocityinLocalSpace (Variables|Default|GetProjectileMovement) (* (Variables|/Game/LetHimCook_Data/Blueprint/Weapon/Ammo/Data/DA_AmmoBase.DA_AmmoBase_C|GetSpeed _asda_ammo_base) "1.000000,0.000000,0.000000"))
  (Transformation|AddWorldRotation (Variables|Default|GetSphere) (Math|Rotator|MakeRotator (Math|Random|RandomFloatinRange 0.0 1.8e+02) (Math|Random|RandomFloatinRange 0.0 1.8e+02) (Math|Random|RandomFloatinRange 0.0 1.8e+02)) false false))

(fn ConstructionScript)