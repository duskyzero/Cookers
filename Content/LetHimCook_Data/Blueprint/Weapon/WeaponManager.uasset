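; WeaponManager initializes weapon and ammo settings from data assets when play begins.
; BeginPlay enables input for the first player controller, then synchronously loads a weapon data asset and an ammo data asset, copying their fields into local variables.
; These cover display info, placement, capacity, weapon object, crosshair widget, and projectile class and speed.
; The graph holds setup only, with no firing or reload logic.
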(event EventBeginPlay
  ;[1 1 1] Initial Values
  (Input|EnableInput (Game|GetPlayerController 0))
  (bind _returnvalue (Utilities|LoadAssetBlocking (Variables|Default|GetDataAsset)))
  (bind _asda_weapon_base (Utilities|Casting|CastToDA_WeaponBase _returnvalue))
  (Variables|Default|SetWeaponName (Variables|/Game/LetHimCook_Data/Blueprint/Weapon/Data/DA_WeaponBase.DA_WeaponBase_C|GetName _asda_weapon_base))
  (Variables|Default|SetWeaponDescription (Variables|/Game/LetHimCook_Data/Blueprint/Weapon/Data/DA_WeaponBase.DA_WeaponBase_C|GetDescription _asda_weapon_base))
  (Variables|Default|SetWeaponTransformLocation (Variables|/Game/LetHimCook_Data/Blueprint/Weapon/Data/DA_WeaponBase.DA_WeaponBase_C|GetTransformLocation _asda_weapon_base))
  (Variables|Default|SetWeaponAmmoCapacity (Variables|/Game/LetHimCook_Data/Blueprint/Weapon/Data/DA_WeaponBase.DA_WeaponBase_C|GetAmmoCapacity _asda_weapon_base))
  (Variables|Default|SetWeaponObject (Variables|/Game/LetHimCook_Data/Blueprint/Weapon/Data/DA_WeaponBase.DA_WeaponBase_C|GetWeaponObject _asda_weapon_base))
  (Variables|Default|SetWeaponCrosshairWidget (Variables|/Game/LetHimCook_Data/Blueprint/Weapon/Data/DA_WeaponBase.DA_WeaponBase_C|GetCrosshairWidget _asda_weapon_base))
  (bind _returnvalue_2 (Utilities|LoadAssetBlocking (Variables|Default|GetAmmoClass)))
  (bind _asda_ammo_base (Utilities|Casting|CastToDA_AmmoBase _returnvalue_2))
  (Variables|Default|SetAmmoName (Variables|/Game/LetHimCook_Data/Blueprint/Weapon/Ammo/Data/DA_AmmoBase.DA_AmmoBase_C|GetName _asda_ammo_base))
  (Variables|Default|SetAmmoSpeed (Variables|/Game/LetHimCook_Data/Blueprint/Weapon/Ammo/Data/DA_AmmoBase.DA_AmmoBase_C|GetSpeed _asda_ammo_base))
  (Variables|Default|SetAmmoMaxAmmo (Variables|/Game/LetHimCook_Data/Blueprint/Weapon/Ammo/Data/DA_AmmoBase.DA_AmmoBase_C|GetMaxAmmo _asda_ammo_base))
  (Variables|Default|SetAmmoProjectileClass (Variables|/Game/LetHimCook_Data/Blueprint/Weapon/Ammo/Data/DA_AmmoBase.DA_AmmoBase_C|GetProjectileClass _asda_ammo_base)))

(fn ConstructionScript)