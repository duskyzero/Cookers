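; BP_DryPistol is a pistol weapon Blueprint that fires projectiles using the ammo count stored on BP_Player.
; BeginPlay creates a crosshair widget, without adding it to the viewport here, and caches the player pawn.
; IA_Shoot spawns the ammo projectile at the Muzzle transform, then WeaponFired decrements and prints the player's pistol ammo.
; At zero ammo, shooting only prints a debug message.
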(event Custom|OnWeaponEquip
  ;[1 1 1] Crosshair NW
  (UserInterface|CreateWidget (Variables|Default|GetWeaponCrosshairWidget) (Game|GetPlayerController 0)))

(event Custom|WeaponFired
  ;[1 1 1] Reduce Ammo
  (bind _output_get (Variables|/Game/LetHimCook_Data/Blueprint/BP_Player.BP_Player_C|SetPistolAmmoCount (stale EventBeginPlay _asbp_player) (- (Variables|/Game/LetHimCook_Data/Blueprint/BP_Player.BP_Player_C|GetPistolAmmoCount (stale EventBeginPlay _asbp_player)) 1)))
  (Development|PrintString (Utilities|String|ToString(Integer) _output_get)))

(event Input|EnhancedActionEvents|EnhancedInputActionIA_Shoot
  (params (ActionValue :type Float%20%28double-precision%29) (ElapsedSeconds :type Float%20%28double-precision%29) (TriggeredSeconds :type Float%20%28double-precision%29) (InputAction :type Input%20Action%20Object%20Reference :default "/Game/LetHimCook_Data/Blueprint/Inputs/IA_Shoot.IA_Shoot"))
  (bind _muzzle (Variables|Default|GetMuzzle))
  (bind _returnvalue (Transformation|GetWorldTransform _muzzle))
  ;[1 1 1] Fire Weapon
  (:Started
    (bind _output_get (Variables|Default|SetIsWeaponEmpty (== (Variables|/Game/LetHimCook_Data/Blueprint/BP_Player.BP_Player_C|GetPistolAmmoCount (stale EventBeginPlay _asbp_player)) 0)))
    (if _output_get
      (Development|PrintString "lmao")
      (else
        (Game|SpawnActorfromClass (Variables|Default|GetAmmoProjectileClass) (Math|Transform|MakeTransform (.location _returnvalue) (.rotation _returnvalue) "1.000000,1.000000,1.000000") "Undefined" "MultiplyWithRoot" 0 0)
        (CallFunction|WeaponFired)))))

(event EventBeginPlay
  ;[1 1 1] Weapon Equip
  (|CallParentFunction)
  (CallFunction|OnWeaponEquip)
  (bind _asbp_player (Utilities|Casting|CastToBP_Player (Game|Player|GetPlayerPawn 0))))

(fn ConstructionScript
  (|CallParentFunction))