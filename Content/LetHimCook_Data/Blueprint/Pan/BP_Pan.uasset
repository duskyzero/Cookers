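; BP_Pan is a pan actor that travels along the spline of the BP_PanPath in the level.
; On BeginPlay it finds the path actor by class and starts the PanMovement timeline.
; Each timeline update maps Alpha to a distance along the spline and sets the pan's world location and rotation to match that point.
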(event Custom|Start%20Moving
  (bind _alpha (Timeline|PanMovement Play)
    (:Update
      (Transformation|SetActorLocationAndRotation (.location (Spline|GetTransformatDistanceAlongSpline (Variables|/Game/LetHimCook_Data/Blueprint/Pan/BP_PanPath.BP_PanPath_C|GetPath (Variables|Default|GetPath)) (Math|Float|Lerp 0.0 (Spline|GetSplineLength (Variables|/Game/LetHimCook_Data/Blueprint/Pan/BP_PanPath.BP_PanPath_C|GetPath (Variables|Default|GetPath))) _alpha) "World" false)) (.rotation (Spline|GetTransformatDistanceAlongSpline (Variables|/Game/LetHimCook_Data/Blueprint/Pan/BP_PanPath.BP_PanPath_C|GetPath (Variables|Default|GetPath)) (Math|Float|Lerp 0.0 (Spline|GetSplineLength (Variables|/Game/LetHimCook_Data/Blueprint/Pan/BP_PanPath.BP_PanPath_C|GetPath (Variables|Default|GetPath))) _alpha) "World" false))))))

(event EventBeginPlay
  (bind _returnvalue (Actor|GetActorOfClass "/Game/LetHimCook_Data/Blueprint/Pan/BP_PanPath.BP_PanPath_C"))
  (Variables|Default|SetPath _returnvalue)
  (CallFunction|StartMoving))

(fn ConstructionScript)