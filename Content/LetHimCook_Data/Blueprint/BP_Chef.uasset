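; BP_Chef is the player character for LetHimCook, handling movement, camera look and weapon switching through Enhanced Input.
; Movement follows the camera's forward and right vectors, and look input also clamps the camera manager's view pitch.
; BeginPlay adds the mapping context, then positions the CurrentWeapon child actor component and loads the first weapon.
; Work-in-progress scrolling swaps that component's class from the Weapons array, wrapping only past the upper end.
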(event Input|EnhancedActionEvents|EnhancedInputActionIA_ChangeWeapon
  (params (ActionValue :type Boolean) (ElapsedSeconds :type Float%20%28double-precision%29) (TriggeredSeconds :type Float%20%28double-precision%29) (InputAction :type Input%20Action%20Object%20Reference :default "/Game/LetHimCook_Data/Blueprint/Inputs/IA_ChangeWeapon.IA_ChangeWeapon"))
  ;[1 1 1] Weapon Scroll (W.I.P)
  (if (>= (+ ActionValue (Variables|Default|GetCurrentWeaponIndex)) (Utilities|Array|Length (Variables|Default|GetWeapons)))
    (Variables|Default|SetCurrentWeaponIndex 0)
    (else
      (Variables|Default|SetCurrentWeaponIndex (+ ActionValue (Variables|Default|GetCurrentWeaponIndex)))))
  (if true
    _
    (else
      _))
  (Development|PrintString (Utilities|String|Append "Current Weapon Index [" (Utilities|String|ToString(Integer) (Variables|Default|GetCurrentWeaponIndex)) "]") true true "(R=1.000000,G=0.170545,B=0.557065,A=1.000000)")
  (ChildActorComponent|SetChildActorClass (Variables|Default|GetCurrentWeapon) (Utilities|Array|Get(acopy) (Variables|Default|GetWeapons) (Variables|Default|GetCurrentWeaponIndex))))

(event Input|EnhancedActionEvents|EnhancedInputActionIA_Movement
  (params (ActionValue :type Vector%202D%20Structure) (ElapsedSeconds :type Float%20%28double-precision%29) (TriggeredSeconds :type Float%20%28double-precision%29) (InputAction :type Input%20Action%20Object%20Reference :default "/Game/LetHimCook_Data/Blueprint/Inputs/IA_Movement.IA_Movement"))
  ;[1 1 1] Movement
  (Pawn|Input|AddMovementInput (Math|Vector|GetRightVector (Variables|Default|GetCamera)) (.x ActionValue) false)
  (Pawn|Input|AddMovementInput (Math|Vector|GetForwardVector (Variables|Default|GetCamera)) (.y ActionValue) false))

(event Input|EnhancedActionEvents|EnhancedInputActionIA_Camera
  (params (ActionValue :type Vector%202D%20Structure) (ElapsedSeconds :type Float%20%28double-precision%29) (TriggeredSeconds :type Float%20%28double-precision%29) (InputAction :type Input%20Action%20Object%20Reference :default "/Game/LetHimCook_Data/Blueprint/Inputs/IA_Camera.IA_Camera"))
  (bind _returnvalue (Game|GetPlayerCameraManager 0))
  ;[1 1 1] Camera
  (Pawn|Input|AddControllerYawInput (.x ActionValue))
  (Pawn|Input|AddControllerPitchInput (.y ActionValue))
  ;[1 1 1] Limit Camera Pitch
  (Variables|/Script/Engine.PlayerCameraManager|SetViewPitchMin _returnvalue -55.0)
  (Variables|/Script/Engine.PlayerCameraManager|SetViewPitchMax _returnvalue 55.0))

(event EventBeginPlay
  ;[1 1 1] Add Mapping Context
  (bind _asplayer_controller (Utilities|Casting|CastToPlayerController (Pawn|GetController)))
  (Utilities|IsValid _asplayer_controller
    (:Is%20Valid
      (Input|AddMappingContext (PlayerController|LocalPlayerSubsystems|GetEnhancedInputLocalPlayerSubsystem _asplayer_controller) "/Game/LetHimCook_Data/Blueprint/Inputs/IMC_LetHimCook.IMC_LetHimCook" 0 "(bIgnoreAllPressedKeysUntilRelease=True,bForceImmediately=False,bNotifyUserSettings=False)")
      ;[1 1 1] Set Location
      (Transformation|SetRelativeLocation (Variables|Default|GetCurrentWeapon) "20.000000,20.000000,-15.000000" false false)
      ;[1 1 1] Set Initial Weapon
      (ChildActorComponent|SetChildActorClass (Variables|Default|GetCurrentWeapon) (Utilities|Array|Get(acopy) (Variables|Default|GetWeapons))))))

(fn ConstructionScript)

(fn IsPlayer?
  (return (Pawn|IsPlayerControlled)))