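; BP_Player is the first-person player Blueprint, handling look, movement, weapon switching and crosshair creation.
; BeginPlay adds the Enhanced Input mapping context, equips the first weapon and creates the crosshair widget.
; IA_ChangeWeapon steps through the Weapons array with wraparound, swapping the Weapon2 child actor class.
; Tick runs a camera-forward debug trace with an unused result and starts walk or idle head-bob shakes by velocity; AmmoControl is empty.
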(event Custom|Tick
  (bind _camera (Variables|Default|GetCamera))
  (bind _returnvalue (Transformation|GetWorldLocation _camera))
  (Collision|LineTraceByChannel _returnvalue (+ _returnvalue (* (Math|Vector|GetForwardVector _camera) 7e+03)) "TraceTypeQuery1" false 0 "ForOneFrame"))

(event Custom|CharacterLoaded
  (UserInterface|CreateWidget "/Game/LetHimCook_Data/Visuals/UI/WB_Crosshair.WB_Crosshair_C" (Game|GetPlayerController 0)))

(event Input|EnhancedActionEvents|EnhancedInputActionIA_ChangeWeapon
  (params (ActionValue :type Float%20%28double-precision%29) (ElapsedSeconds :type Float%20%28double-precision%29) (TriggeredSeconds :type Float%20%28double-precision%29) (InputAction :type Input%20Action%20Object%20Reference :default "/Game/LetHimCook_Data/Blueprint/Inputs/IA_ChangeWeapon.IA_ChangeWeapon"))
  (if (>= (+ (Math|Float|Truncate (Math|Float|Absolute(Float) ActionValue)) (Variables|Default|GetCurrent%20Weapon%20Index)) (Utilities|Array|Length (Variables|Default|GetWeapons)))
    (Variables|Default|SetCurrent%20Weapon%20Index 0)
    (else
      (Variables|Default|SetCurrent%20Weapon%20Index (+ (Math|Float|Truncate (Math|Float|Absolute(Float) ActionValue)) (Variables|Default|GetCurrent%20Weapon%20Index)))))
  (ChildActorComponent|SetChildActorClass (Variables|Default|GetWeapon2) (Utilities|Array|Get(acopy) (Variables|Default|GetWeapons) (Variables|Default|GetCurrent%20Weapon%20Index))))

(event Input|EnhancedActionEvents|EnhancedInputActionIA_Movement
  (params (ActionValue :type Vector%202D%20Structure) (ElapsedSeconds :type Float%20%28double-precision%29) (TriggeredSeconds :type Float%20%28double-precision%29) (InputAction :type Input%20Action%20Object%20Reference :default "/Game/LetHimCook_Data/Blueprint/Inputs/IA_Movement.IA_Movement"))
  ;[1 1 1] Movement
  (Pawn|Input|AddMovementInput (Math|Vector|GetRightVector (Variables|Default|GetCamera)) (.x ActionValue) false)
  (Pawn|Input|AddMovementInput (Math|Vector|GetForwardVector (Variables|Default|GetCamera)) (.y ActionValue) false))

(event Input|EnhancedActionEvents|EnhancedInputActionIA_Camera
  (params (ActionValue :type Vector%202D%20Structure) (ElapsedSeconds :type Float%20%28double-precision%29) (TriggeredSeconds :type Float%20%28double-precision%29) (InputAction :type Input%20Action%20Object%20Reference :default "/Game/LetHimCook_Data/Blueprint/Inputs/IA_Camera.IA_Camera"))
  ;[1 1 1] Add Camera Movement
  (Pawn|Input|AddControllerYawInput (.x ActionValue))
  (Pawn|Input|AddControllerPitchInput (.y ActionValue)))

(event EventBeginPlay
  ;[1 1 1] Add Mapping Context
  (bind _asplayer_controller (Utilities|Casting|CastToPlayerController (Pawn|GetController)))
  (Utilities|IsValid _asplayer_controller
    (:Is%20Valid
      (Input|AddMappingContext (PlayerController|LocalPlayerSubsystems|GetEnhancedInputLocalPlayerSubsystem _asplayer_controller) "/Game/LetHimCook_Data/Blueprint/Inputs/IMC_LetHimCook.IMC_LetHimCook" 0 "(bIgnoreAllPressedKeysUntilRelease=True,bForceImmediately=False,bNotifyUserSettings=False)")
      ;[1 1 1] Set Initial Weapon
      (ChildActorComponent|SetChildActorClass (Variables|Default|GetWeapon2) (Utilities|Array|Get(acopy) (Variables|Default|GetWeapons)))
      (CallFunction|CharacterLoaded))))

(event EventTick
  (params (DeltaSeconds :type Float%20%28single-precision%29))
  (bind _returnvalue (Game|GetPlayerCameraManager 0))
  ;[1 1 1] Camera Bobbing
  (CallFunction|Tick)
  (if (> (Math|Vector|VectorLength (Transformation|GetVelocity)) 0.0)
    (Class|LegacyCameraShake|StartLegacyCameraShake _returnvalue "/Game/LetHimCook_Data/Blueprint/CamershakePresets/BP_HeadBobWalk.BP_HeadBobWalk_C" 1.0 "CameraLocal" "0, 0, 0")
    (else
      (Class|LegacyCameraShake|StartLegacyCameraShake _returnvalue "/Game/LetHimCook_Data/Blueprint/CamershakePresets/BP_HeadBobIdle.BP_HeadBobIdle_C" 1.0 "CameraLocal" "0, 0, 0"))))

(fn ConstructionScript)

(fn AmmoControl
  (params (CurrentAmmo :type Integer)))