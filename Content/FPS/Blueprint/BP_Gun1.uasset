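; BP_Gun1 is a gun Blueprint for an FPS that enables player input on itself at BeginPlay.
; When the Enhanced Input shoot action starts, it line traces on the Visibility channel forward from its Arrow component, with timed debug drawing.
; It then plays a world camera shake centered on the gun.
; The trace result is not yet used, so shots apply no damage or impact effects.
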(event Input|EnhancedActionEvents|EnhancedInputActionIA_Shoot
  (params (ActionValue :type Float%20%28double-precision%29) (ElapsedSeconds :type Float%20%28double-precision%29) (TriggeredSeconds :type Float%20%28double-precision%29) (InputAction :type Input%20Action%20Object%20Reference :default "/Game/FPS/Blueprint/Inputs/IA_Shoot.IA_Shoot"))
  (bind _arrow (Variables|Default|GetArrow))
  (bind _returnvalue (Transformation|GetWorldTransform _arrow))
  (:Started
    (bind _outhit (Collision|LineTraceByChannel (.location _returnvalue) (+ (.location _returnvalue) (* (Math|Vector|GetForwardVector (.rotation _returnvalue)) 5e+03)) "TraceTypeQuery1" false 0 "ForDuration"))
    (Camera|PlayWorldCameraShake "/Game/FPS/Blueprint/Inputs/BP_ShootCameraShake.BP_ShootCameraShake_C" (Transformation|GetActorLocation) 0.0 3e+03)))

(event EventBeginPlay
  (Input|EnableInput (Game|GetPlayerController 0)))

(fn ConstructionScript)