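; FPSChar is a first-person player character that adds a crosshair HUD widget on BeginPlay and handles look, movement and firing.
; Movement and look are wired through both legacy axis events, which move along camera vectors, and Enhanced Input actions, which use actor vectors.
; Fire runs a debug-drawn visibility line trace forward from the camera and plays a world camera shake; the trace result is unused.
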(event EventBeginPlay
  ;[1 1 1] Crosshair
  (bind _returnvalue (UserInterface|CreateWidget "/Game/UI/WB_HUD.WB_HUD_C"))
  (UserInterface|Viewport|AddtoViewport _returnvalue 0))

(event Input|ActionEvents|InputActionFire
  (params (Key :type Key%20Structure :default "None"))
  (bind _camera (Variables|Default|GetCamera))
  (bind _returnvalue (Transformation|GetWorldTransform _camera))
  (:Pressed
    (Collision|LineTraceByChannel (.location _returnvalue) (+ (.location _returnvalue) (* (Math|Vector|GetForwardVector (.rotation _returnvalue)) 5e+03)) "TraceTypeQuery1" false 0 "ForDuration")
    (Camera|PlayWorldCameraShake "/Game/FPS/Blueprint/Inputs/BP_ShootCameraShake.BP_ShootCameraShake_C" (Transformation|GetActorLocation) 0.0 3e+03)))

(event Input|AxisEvents|InputAxisTurn
  (params (AxisValue :type Float%20%28single-precision%29))
  ;[1 1 1] Camera
  (Pawn|Input|AddControllerYawInput AxisValue))

(event Input|AxisEvents|InputAxisLookUp
  (params (AxisValue :type Float%20%28single-precision%29))
  ;[1 1 1] Camera
  (Pawn|Input|AddControllerPitchInput AxisValue))

(event Input|AxisEvents|InputAxisMoveForward
  (params (AxisValue :type Float%20%28single-precision%29))
  ;[1 1 1] Movement
  (Pawn|Input|AddMovementInput (Math|Vector|GetForwardVector (Variables|Default|GetCamera)) AxisValue false))

(event Input|AxisEvents|InputAxisMoveRight
  (params (AxisValue :type Float%20%28single-precision%29))
  ;[1 1 1] Movement
  (Pawn|Input|AddMovementInput (Math|Vector|GetRightVector (Variables|Default|GetCamera)) AxisValue false))

(event Input|EnhancedActionEvents|EnhancedInputActionIA_Camera
  (params (ActionValue :type Vector%202D%20Structure) (ElapsedSeconds :type Float%20%28double-precision%29) (TriggeredSeconds :type Float%20%28double-precision%29) (InputAction :type Input%20Action%20Object%20Reference :default "/Game/FPS/Blueprint/Inputs/IA_Camera.IA_Camera"))
  (Pawn|Input|AddControllerYawInput (.x ActionValue))
  (Pawn|Input|AddControllerPitchInput (.y ActionValue)))

(event Input|EnhancedActionEvents|EnhancedInputActionIA_Movement
  (params (ActionValue :type Vector%202D%20Structure) (ElapsedSeconds :type Float%20%28double-precision%29) (TriggeredSeconds :type Float%20%28double-precision%29) (InputAction :type Input%20Action%20Object%20Reference :default "/Game/FPS/Blueprint/Inputs/IA_Movement.IA_Movement"))
  (Pawn|Input|AddMovementInput (Transformation|GetActorRightVector) (.x ActionValue) false)
  (Pawn|Input|AddMovementInput (Transformation|GetActorForwardVector) (.y ActionValue) false))

(fn ConstructionScript)